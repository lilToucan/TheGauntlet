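; Player character Blueprint for the Gauntlet game that handles pause input and draws a debug sphere showing its overlap range every tick.
; The pause action pushes a pause menu through the player controller's HUD widget, caches it, shows the cursor and has the game instance pause.
; Pressing it again while paused calls the cached menu's resume function and clears the character's paused flag.
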(event `self.ReceiveTick`
  (params (DeltaSeconds :type "Float (single-precision)"))
  (`KismetSystemLibrary.DrawDebugSphere` (`self.K2_GetActorLocation`) (`self.OverlapSphereRange`)))

(event `EnhancedInput|/Game/TheGauntlet_Game/Core/Inputs/Actions/IA_PauseGame`
  (params (ActionValue :type Boolean) (ElapsedSeconds :type "Float (double-precision)") (TriggeredSeconds :type "Float (double-precision)") (InputAction :type "InputAction Object Reference" :default "/Game/TheGauntlet_Game/Core/Inputs/Actions/IA_PauseGame.IA_PauseGame"))
  (bind _pausemenu (`self.PauseMenu`))
  (:`Started`
    (if (`self.IsPaused`)
      (`/Engine/EditorBlueprintResources/StandardMacros.IsValid` _pausemenu
        (:`Is Valid`
          (`/Game/TheGauntlet_Game/Blueprints/UI/Widgets/WBP_PauseMenu.ResumeFunction` _pausemenu)
          (set `self.IsPaused` false)))
      (else
        (bind _asbp_gauntlet_player_controller (cast `/Game/TheGauntlet_Game/Core/BP_GauntletPlayerController` (`GameplayStatics.GetPlayerController` 0)))
        (bind _returnvalue (`/Game/TheGauntlet_Game/Blueprints/UI/Widgets/WBP_HUD.PushWidget` (`/Game/TheGauntlet_Game/Core/BP_GauntletPlayerController.HudWidget` _asbp_gauntlet_player_controller) "/Game/TheGauntlet_Game/Blueprints/UI/Widgets/WBP_PauseMenu.WBP_PauseMenu_C"))
        (bind _aswbp_pause_menu (cast `/Game/TheGauntlet_Game/Blueprints/UI/Widgets/WBP_PauseMenu` _returnvalue))
        (set `self.PauseMenu` _aswbp_pause_menu)
        (set `self.IsPaused` true)
        (set `PlayerController.bShowMouseCursor` true (`GameplayStatics.GetPlayerController` 0))
        (bind _asbp_gauntlet_game_instance (cast `/Game/TheGauntlet_Game/Core/BP_GauntletGameInstance` (`GameplayStatics.GetGameInstance`)))
        (`TheGauntlet_GameInstance.PauseGame` _asbp_gauntlet_game_instance)))))

(fn `UserConstructionScript`)